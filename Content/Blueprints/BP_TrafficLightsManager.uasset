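; Traffic light manager that lights one BP_TraffictLight actor at a time in a repeating three-step cycle, starting at BeginPlay.
; Recolor blacks out the current light, advances the index and colors the next from the ColorSettings map via an enum key.
; It then resets its own looping timer by function name, giving each step its own duration.
; Light order depends on GetAllActorsOfClass, which runs on every change.
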(event `self.ReceiveBeginPlay`
  (`self.Recolor`))

(event `Recolor`
  (bind _outactors (`GameplayStatics.GetAllActorsOfClass` "/Game/Blueprints/BP_TraffictLight.BP_TraffictLight_C"))
  (bind _output (`|GetArrayItem` _outactors (`self.CurrentIndex`)))
  (`/Game/Blueprints/BP_TraffictLight.ChangeColor` :`self` _output)
  (set `self.CurrentIndex` (mod (+ (`self.CurrentIndex`) 1) 3))
  (`/Game/Blueprints/BP_TraffictLight.ChangeColor` _output (`BlueprintMapLibrary.Map_Find` (`.ColorMap_24_B0963E464DEDED4DE63930B32408AE9C` (break `/Game/Blueprints/S_LIghtColor` (`self.ColorSettings`))) (`|GetArrayItem` (`|MakeArray` "NewEnumerator1" "NewEnumerator0" "NewEnumerator2" :!type "/Game/Blueprints/E_LightColor Enum") (`self.CurrentIndex`))))
  (`|ExecutionSequence`
    (:`then_0`
      (if (== (`self.CurrentIndex`) 0)
        (`KismetSystemLibrary.K2_SetTimer` null "Recolor" 1.0 true)))
    (:`then_1`
      (if (== (`self.CurrentIndex`) 1)
        (`KismetSystemLibrary.K2_SetTimer` null "Recolor" 5.0 true)))
    (:`then_2`
      (if (== (`self.CurrentIndex`) 2)
        (`KismetSystemLibrary.K2_SetTimer` null "Recolor" 3.0 true)))))

(fn `UserConstructionScript`)